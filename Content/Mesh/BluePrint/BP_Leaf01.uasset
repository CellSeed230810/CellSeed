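; BP_Leaf01 is a leaf Blueprint that animates growth by stretching a SplineMesh along a Spline.
; BeginPlay or the Player01 event randomizes tangent strength and plays a timeline that drives Distance.
; PlantUpdate uses Distance to move the mesh end along the spline, lengthen both tangents and scale both ends uniformly.
; The construction script runs the same update, shaping the mesh from the current Distance.
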(event EventBeginPlay
  (Variables|Default|SetRandom_Dis (Math|Random|RandomFloatinRange 1.0 1.0))
  (Variables|Default|SetRandom_Tang (Math|Random|RandomFloatinRange 0.8 1.2))
  (bind _新建轨道_0 (Timeline|时间轴_0 PlayFromStart)
    (:Update
      (Variables|Default|SetDistance (* _新建轨道_0 (Variables|Default|GetRandom_Dis)))
      (CallFunction|PlantUpdate))))

(event EventPlayer01
  (Variables|Default|SetRandom_Dis (Math|Random|RandomFloatinRange 1.0 1.0))
  (Variables|Default|SetRandom_Tang (Math|Random|RandomFloatinRange 0.8 1.2))
  (bind _新建轨道_0 (Timeline|时间轴_0 PlayFromStart)
    (:Update
      (Variables|Default|SetDistance (* _新建轨道_0 (Variables|Default|GetRandom_Dis)))
      (CallFunction|PlantUpdate))))

(fn ConstructionScript
  (CallFunction|PlantUpdate))

(fn PlantUpdate
  (bind _splinemesh (Variables|Default|GetSplineMesh))
  (bind _spline (Variables|Default|GetSpline))
  (bind _distance (Variables|Default|GetDistance))
  (bind _distance_2 (Variables|Default|GetDistance))
  (bind _distance_3 (Variables|Default|GetDistance))
  (bind _random_tang (Variables|Default|GetRandom_Tang))
  (bind _returnvalue (Math|Vector2D|MakeVector2D _distance_2 _distance_2))
  (bind _returnvalue_2 (Math|Float|Lerp 3e+01 1e+02 _distance_3))
  (bind _returnvalue_3 (Spline|GetSplineLength _spline))
  (bind _returnvalue_4 (* _returnvalue_2 _random_tang))
  (bind _returnvalue_5 (* _returnvalue_3 _distance))
  (SplineMesh|SetStartandEnd _splinemesh (Spline|GetLocationatDistanceAlongSpline _spline 0.0 "Local") (* (Spline|GetDirectionatDistanceAlongSpline _spline 0.0 "Local") _returnvalue_4) (Spline|GetLocationatDistanceAlongSpline _spline _returnvalue_5 "Local") (* (Spline|GetDirectionatDistanceAlongSpline _spline _returnvalue_5 "Local") _returnvalue_4) true :!class /Script/Engine.SplineMeshComponent)
  (SplineMesh|SetStartScale _splinemesh _returnvalue true :!class /Script/Engine.SplineMeshComponent)
  (SplineMesh|SetEndScale _splinemesh _returnvalue true :!class /Script/Engine.SplineMeshComponent))