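; Space backdrop actor that moves meshes along a spline, with a scroll child actor trailing them and a delayed background sound.
; Construction script spawns scaled spline mesh components from a configurable mesh and material.
; Tick advances each by its speed plus jitter, orients it along the spline, offsets the scroll from it and wraps near the end; the construction-time speed randomiser is unwired.
; BeginPlay optionally starts the scroll animation after a delay.
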(event EventBeginPlay
  (Utilities|FlowControl|Sequence
    (:then_0
      (if (Variables|Default|GetPlay_Shuoming)
        (Utilities|FlowControl|Delay (Variables|Default|GetDelay_Shuoming))
        (bind _asbp_scroll (Utilities|Casting|CastToBP_Scroll (Variables|/Script/Engine.ChildActorComponent|GetChildActor (Variables|Default|GetBP_Scroll))))
        (Variables|/Game/UIClara/BP/BP_Scroll.BP_Scroll_C|SetPlay_Ani _asbp_scroll true)))
    (:then_1
      (Utilities|FlowControl|Delay (Variables|Default|GetDelaySound))
      (Audio|Components|Audio|Play (Variables|Default|GetS_SpaceBackground) 0.0))))

(event EventTick
  (params (DeltaSeconds :type Float%20%28single-precision%29))
  (bind _spline (Variables|Default|GetSpline))
  (for (_ _array_index) (Variables|Default|Getniaoooo)
    (Utilities|Array|SetArrayElem (Variables|Default|GetDistanceAlongSpline_shuzu) _array_index (+ (Math|Random|RandomFloatinRange (Utilities|Array|Get(acopy) (Variables|Default|GetSpeed_shuzu) _array_index) (+ (Utilities|Array|Get(acopy) (Variables|Default|GetSpeed_shuzu) _array_index) 0.5)) (Utilities|Array|Get(acopy) (Variables|Default|GetDistanceAlongSpline_shuzu) _array_index)))
    (Transformation|SetRelativeLocationAndRotation (Utilities|Array|Get(acopy) (Variables|Default|Getniaoooo) _array_index) (+ (Spline|GetLocationatDistanceAlongSpline _spline (Utilities|Array|Get(acopy) (Variables|Default|GetDistanceAlongSpline_shuzu) _array_index) "Local") "0, 0, 0") (Math|Rotator|MakeRotator (.roll (Math|Conversions|RotationFromXVector (Spline|GetDirectionatDistanceAlongSpline _spline (Utilities|Array|Get(acopy) (Variables|Default|GetDistanceAlongSpline_shuzu) _array_index) "Local"))) (.pitch (Math|Conversions|RotationFromXVector (Spline|GetDirectionatDistanceAlongSpline _spline (Utilities|Array|Get(acopy) (Variables|Default|GetDistanceAlongSpline_shuzu) _array_index) "Local"))) (+ (.yaw (Math|Conversions|RotationFromXVector (Spline|GetDirectionatDistanceAlongSpline _spline (Utilities|Array|Get(acopy) (Variables|Default|GetDistanceAlongSpline_shuzu) _array_index) "Local"))) 1.8e+02)) false false)
    (Transformation|SetWorldLocation (Variables|Default|GetBP_Scroll) (- (Transformation|GetWorldLocation (Utilities|Array|Get(acopy) (Variables|Default|Getniaoooo) _array_index)) "500.000000,500.000000,0.000000") false false)
    (if (Math|Float|NearlyEqual(Float) (Utilities|Array|Get(acopy) (Variables|Default|GetDistanceAlongSpline_shuzu) _array_index) (Spline|GetSplineLength _spline) (Math|Random|RandomFloatinRange (Utilities|Array|Get(acopy) (Variables|Default|GetSpeed_shuzu) _array_index) (+ (Utilities|Array|Get(acopy) (Variables|Default|GetSpeed_shuzu) _array_index) 0.5)))
      (Utilities|Array|SetArrayElem (Variables|Default|GetDistanceAlongSpline_shuzu) _array_index 0.0))))

(fn ConstructionScript
  (bind _spline (Variables|Default|GetSpline))
  (bind _returnvalue (Spline|GetDirectionatDistanceAlongSpline _spline 0.0 "Local"))
  (bind _returnvalue_2 (Math|Conversions|RotationFromXVector _returnvalue))
  (for _index (range 0 (Variables|Default|GetNUM))
    (bind _returnvalue_3 (AddComponent|AddSplineMeshComponent false))
    (Utilities|Array|AddUnique (Variables|Default|GetDistanceAlongSpline_shuzu) 5e+02)
    (Utilities|Array|AddUnique (Variables|Default|Getniaoooo) _returnvalue_3)
    (Utilities|Array|AddUnique :TargetArray (Variables|Default|GetNiao_XZ))
    (Components|StaticMesh|SetStaticMesh _returnvalue_3 (Variables|Default|GetMesh))
    (Rendering|Material|SetMaterial _returnvalue_3 0 (Variables|Default|Getmaterial))
    (Transformation|SetRelativeLocation _returnvalue_3 "0, 0, 0" false false)
    (Transformation|SetRelativeLocation _returnvalue_3 (+ (Spline|GetLocationatDistanceAlongSpline _spline 0.0 "Local") "0, 0, 0") false false)
    (Transformation|SetRelativeRotation _returnvalue_3 (Math|Rotator|MakeRotator (.roll _returnvalue_2) (.pitch _returnvalue_2) (.yaw _returnvalue_2)) false false)
    (Transformation|AddLocalRotation _returnvalue_3 (Math|Rotator|MakeRotator 0.0 0.0 -9e+01) false false)
    (Transformation|SetRelativeScale3D _returnvalue_3 "20.000000,1.000000,1.000000")
    (Transformation|AttachComponentToComponent _returnvalue_3 "None" "KeepRelative" "KeepRelative" "KeepRelative" true)))