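; BP_Scroll is a world-space scroll panel that shows a Title and Meaning in a WBP_DescriptionPanel widget created at BeginPlay.
; Tick yaws its Rotation and Cube components with the player camera so the panel follows the view.
; After a Delay, Tick plays a timeline when PlayAni is set, fading in the widget and its frame components through tint opacity.
; PlayUI toggles the visibility of those components.
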(event EventBeginPlay
  (Class|WidgetComponent|SetTintColorandOpacity (Variables|Default|GetDescription_Kuang5) (Utilities|Struct|MakeLinearColor 1.0 1.0 1.0 0.0))
  (Rendering|SetVisibility (Variables|Default|GetDescriptionFrontFrame) true false)
  ;[1 1 1] Description Widget
  (bind _returnvalue (UserInterface|CreateWidget "/Game/UIClara/BP/Widget/WBP_DescriptionPanel.WBP_DescriptionPanel_C"))
  (bind _output_get (Variables|Default|SetDescriptionPanelWidget _returnvalue))
  (UserInterface|SetWidget (Variables|Default|GetDescriptionWidget) _output_get)
  (Rendering|Components|TextRender|SetText (Variables|/Game/UIClara/BP/Widget/WBP_DescriptionPanel.WBP_DescriptionPanel_C|GetTitleText (Variables|Default|GetDescriptionPanelWidget)) (Utilities|Text|ToText(String) (Variables|Default|GetTitle)))
  (Rendering|Components|TextRender|SetText (Variables|/Game/UIClara/BP/Widget/WBP_DescriptionPanel.WBP_DescriptionPanel_C|GetDescriptionText (Variables|Default|GetDescriptionPanelWidget)) (Utilities|Text|ToText(String) (Variables|Default|GetMeaning))))

(event EventTick
  (params (DeltaSeconds :type Float%20%28single-precision%29))
  (bind _returnvalue (Game|GetPlayerCameraManager 0))
  (bind _returnvalue_2 (Camera|GetCameraRotation _returnvalue))
  (Utilities|FlowControl|Sequence
    (:then_0
      (Transformation|SetWorldRotation (Variables|Default|GetRotation) (Math|Rotator|MakeRotator 0.0 0.0 (+ (.yaw _returnvalue_2) 1.8e+02)) false false)
      (Transformation|SetWorldRotation (Variables|Default|GetCube) (Math|Rotator|MakeRotator 0.0 0.0 (.yaw _returnvalue_2)) false false))
    (:then_1
      (Utilities|FlowControl|Delay (Variables|Default|GetDelay))
      (if (Variables|Default|GetPlay_Ani)
        (bind _新建轨道_0 (Timeline|时间轴 Play)
          (:Update
            (Class|WidgetComponent|SetTintColorandOpacity (Variables|Default|GetDescriptionWidget) (Utilities|Struct|MakeLinearColor 1.0 1.0 1.0 (Math|Float|Lerp 0.0 1.0 _新建轨道_0))))
          (:Finished
            (Class|WidgetComponent|SetTintColorandOpacity (Variables|Default|GetDescriptionBackFrame) (Utilities|Struct|MakeLinearColor 1.0 1.0 1.0 0.0))))))))

(event EventPlayUI
  (Rendering|ToggleVisibility (Variables|Default|GetDescriptionFrontFrame) false))

(fn ConstructionScript)